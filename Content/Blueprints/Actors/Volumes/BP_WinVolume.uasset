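; BP_WinVolume is a volume actor that ends the level when the player overlaps it.
; It completes the level only if AnyCrystalRemaining is true, meaning more than two BP_Crystal actors exist.
; Completion checks the current level against the LevelName array: the last entry opens the hard-coded Level1, while any other quits the game.
; GetNextLevelName, which returns the following array entry, is unused.
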(event Collision|EventActorBeginOverlap
  (params (OtherActor :type Actor%20Object%20Reference))
  (Utilities|IsPlayer OtherActor
    (:Is%20Player
      (if (CallFunction|AnyCrystalRemaining)
        (LevelManagement|CompleteLevel)))))

(fn ConstructionScript)

(fn AnyCrystalRemaining
  (bind _outactors (Actor|GetAllActorsOfClass "/Game/Blueprints/Actors/Collectableses/BP_Crystal.BP_Crystal_C"))
  (return (> (Utilities|Array|Length _outactors) 2)))

(fn CompleteLevel
  (if (LevelManagement|IsFinalLevel)
    (LevelManagement|LoadNextLevel)
    (else
      (Game|QuitGame 0 "Quit" false))))

(fn GetCurrentLevelIndex
  (bind _returnvalue (Game|GetCurrentLevelName true))
  (return (Utilities|Array|FindItem (Variables|Default|GetLevel%20Name) (Utilities|String|StringToName _returnvalue))))

(fn IsFinalLevel
  (return (== (Utilities|Array|LastIndex (Variables|Default|GetLevel%20Name)) (LevelManagement|GetCurrentLevelIndex))))

(fn LoadNextLevel
  (Game|OpenLevel(byName) "Level1"))

(fn GetNextLevelName
  (return (Utilities|Array|Get(acopy) (Variables|Default|GetLevel%20Name) (+ (LevelManagement|GetCurrentLevelIndex) 1))))